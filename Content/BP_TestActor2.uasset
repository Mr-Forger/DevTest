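; BP_TestActor2 is a test actor that bridges an on-screen LLM chat widget and a Llama component.
; BeginPlay creates WBP_LlmChat with a self reference and loads the model.
; TextInputFromLlmChat inserts text as a templated prompt; finished responses return to the widget as non-player messages.
; Tokens, errors and load success print for debugging; the node setting an Unreal-expert system prompt is unconnected.
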(event OnModelLoaded(Llama)
  (params (ModelName :type String))
  (Development|PrintString "LLM Model LOADED SUCCESSFULLY!" true true "(R=0.000000,G=0.660000,B=1.000000,A=1.000000)" 1e+01))

(event OnTokenGenerated(Llama)
  (params (Token :type String))
  (Development|PrintString Token true true "(R=0.000000,G=0.660000,B=1.000000,A=1.000000)" 1e+01))

(event OnResponseGenerated(Llama)
  (params (Response :type String))
  (bind _llmchatwidgetref (Variables|Default|GetLlmChatWidgetRef))
  (Utilities|IsValid _llmchatwidgetref
    (:Is%20Valid
      (Class|LlmChat|AddMessagetoUI _llmchatwidgetref Response false)
      (Development|PrintString Response true true "(R=1.000000,G=0.838720,B=0.270461,A=1.000000)" 1e+01))))

(event OnError(Llama)
  (params (ErrorMessage :type String) (ErrorCode :type Integer))
  (Development|PrintString (Utilities|String|Append ErrorMessage (Utilities|String|ToString(Integer) ErrorCode)) true true "(R=0.000000,G=0.660000,B=1.000000,A=1.000000)" 1e+01))

(event Custom|TextInputFromLlmChat
  (params (Inputs :type String))
  (Class|LlamaComponent|InsertTemplatedPrompt (Variables|Default|GetLlama) Inputs "User" false true))

(event EventBeginPlay
  (bind _returnvalue (UserInterface|CreateWidget "/Game/Widget/WBP_LlmChat.WBP_LlmChat_C" 0 self))
  (bind _output_get (Variables|Default|SetLlmChatWidgetRef _returnvalue))
  (UserInterface|Viewport|AddtoViewport _output_get 0)
  (Class|LlamaComponent|LoadModel (Variables|Default|GetLlama) true))

(event Collision|EventActorBeginOverlap
  (params (OtherActor :type Actor%20Object%20Reference)))

(event EventTick
  (params (DeltaSeconds :type Float%20%28single-precision%29)))

(fn ConstructionScript)